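; BP_FT_AnimNotify is an animation notify that plays walking footstep sounds matched to the surface beneath the character.
; When received, it traces 200 units down from the mesh owner's location along its inverted up vector on the Visibility channel.
; The hit's physical surface selects the Wood, Stone, Water or Dirt sound.
; Sounds play at world origin rather than at the hit or owner location.
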(fn `Received_Notify`
  (params (MeshComp :type "SkeletalMeshComponent Object Reference") (Animation :type "AnimSequenceBase Object Reference") (EventReference :type "AnimNotifyEventReference Structure (by ref)"))
  (returns (ReturnValue :type Boolean))
  (bind _returnvalue (`ActorComponent.GetOwner` MeshComp))
  (bind _returnvalue_2 (`Actor.K2_GetActorLocation` _returnvalue))
  (bind (_outhit _returnvalue_3) (`KismetSystemLibrary.LineTraceSingle` _returnvalue_2 (+ _returnvalue_2 (* (`Actor.GetActorUpVector` _returnvalue) -200.0)) "TraceTypeQuery1"))
  (if _returnvalue_3
    (switch `EPhysicalSurface` (`GameplayStatics.GetSurfaceType` _outhit)
      (:`SurfaceType1`
        (`GameplayStatics.PlaySoundAtLocation` "/Game/Audio/MC/MC_FT_Wood/MC_FT_Wood_Walk.MC_FT_Wood_Walk" (0.0 0.0 0.0) (struct) 1.0 1.0 0.0 null null null null))
      (:`SurfaceType2`
        (`GameplayStatics.PlaySoundAtLocation` "/Game/Audio/MC/MC_FT_Stone/MC_FT_Stone_Walk.MC_FT_Stone_Walk" (0.0 0.0 0.0) (struct) 1.0 1.0 0.0 null null null null))
      (:`SurfaceType3`
        (`GameplayStatics.PlaySoundAtLocation` "/Game/Audio/MC/MC_FT_Water/MC_FT_Water_Walk.MC_FT_Water_Walk" (0.0 0.0 0.0) (struct) 1.0 1.0 0.0 null null null null))
      (:`SurfaceType4`
        (`GameplayStatics.PlaySoundAtLocation` "/Game/Audio/MC/MC_FT_Dirt/MC_FT_Dirt_Walk.MC_FT_Dirt_Walk" (0.0 0.0 0.0) (struct) 1.0 1.0 0.0 null null null null))))
  (return false))